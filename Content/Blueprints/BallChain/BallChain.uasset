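; BallChain is a side-scrolling melee character that moves along X, faces left or right with its velocity, and can be stunned or defeated.
; Its hitbox overlap deals fixed damage to other BallChain actors through ReceiveAttack, which jumps the Locomotion state machine to stunned or dead states.
; A timer follows each stun, and defeat disables capsule collision.
; SetHitboxCollision ignores its argument and always enables query collision.
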(event OnComponentBeginOverlap(Hitbox)
  (params (OverlappedComponent :type Primitive%20Component%20Object%20Reference) (OtherActor :type Actor%20Object%20Reference) (OtherComp :type Primitive%20Component%20Object%20Reference) (OtherBodyIndex :type Integer) (bFromSweep :type Boolean) (SweepResult :type Hit%20Result%20Structure%20%28by%20ref%29))
  (bind _asball_chain (Utilities|Casting|CastToBallChain OtherActor))
  (CallFunction|ReceiveAttack _asball_chain 25.0))

(event EventBeginPlay
  (CallFunction|SetHitboxCollision false)
  (Variables|Default|SetCurrentHealth (Variables|Default|GetMaxHealth)))

(event Collision|EventActorBeginOverlap
  (params (OtherActor :type Actor%20Object%20Reference)))

(event EventTick
  (params (DeltaSeconds :type Float%20%28single-precision%29))
  (bind _returnvalue (Pawn|GetController))
  (|CallParentFunction 0.0)
  (Math|Float|CompareFloat (.X (Math|Vector|BreakVector (Variables|/Script/Engine.MovementComponent|GetVelocity (Pawn|GetMovementComponent)))) 0.0
    (:>
      ;[0 0.4745 1] Look Right
      (Utilities|IsValid _returnvalue
        (:Is%20Valid
          (Pawn|SetControlRotation _returnvalue (Math|Rotator|MakeRotator 0.0 0.0 0.0)))))
    (:<
      ;[0 0.4745 1] Look Left
      (Utilities|IsValid 0
        (:Is%20Valid
          (Pawn|SetControlRotation (Pawn|GetController) (Math|Rotator|MakeRotator 0.0 0.0 1.8e+02)))))))

(event Input|AxisEvents|InputAxisForward
  (params (AxisValue :type Float%20%28single-precision%29))
  (Pawn|Input|AddMovementInput "1.000000,0.000000,0.000000" AxisValue false))

(fn ConstructionScript)

(fn ReceiveAttack
  (params (Damage :type Float%20%28double-precision%29))
  (if (not (Variables|Default|GetIsDefeated))
    (Variables|Default|SetCurrentHealth (- (Variables|Default|GetCurrentHealth) Damage))
    (if (<= (Variables|Default|GetCurrentHealth) 0.0)
      (Class|PaperZDAnimInstance|JumptoNode (Class|PaperZDCharacter|GetAnimInstance) "Dead" "Locomotion")
      (Variables|Default|SetIsDefeated true)
      (Collision|SetCollisionEnabled (Variables|Default|GetCapsuleComponent) "NoCollision")
      (else
        (Variables|Default|SetIsStunned true)
        (Class|PaperZDAnimInstance|JumptoNode (Class|PaperZDCharacter|GetAnimInstance) "JumpStunned" "Locomotion")
        (Utilities|Time|SetTimerbyEvent (EventDispatchers|CreateEvent :!event ClearStun) (Variables|Default|GetStunLength))))))

(fn ClearStun
  (Variables|Default|SetIsStunned false))

(fn SetHitboxCollision
  (params (SetActive :type Boolean))
  (if true
    (Collision|SetCollisionEnabled (Variables|Default|GetHitbox) "QueryOnly")
    (else
      (Collision|SetCollisionEnabled (Variables|Default|GetHitbox) "NoCollision"))))