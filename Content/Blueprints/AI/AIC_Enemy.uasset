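; AI controller for the BallChain enemy, running its behavior tree and controlling its facing.
; On possess it mirrors the pawn's stun state into the blackboard.
; A temporary aggro system on BeginPlay sets the player's BP_Warrior as attack target.
; Each tick it focuses toward the target along world X only, holding the current facing when attacking, stunned or without a target.
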(event Custom|OnStunStateChanged
  (params (isStunned :type Boolean))
  ;[1 1 1] connects isStunned to blackboard
  (AI|Components|Blackboard|SetValueasBool (Variables|Default|GetBlackboard) (Variables|Default|GetisStunnedKey) isStunned))

(event EventBeginPlay
  (Class|AIController|UseBlackboard "/Game/Blueprints/AI/BB_BC.BB_BC")
  (AI|RunBehaviorTree "/Game/Blueprints/AI/BT_BC.BT_BC")
  ;[1 1 1] Temporary Aggro System
  (bind _asbp_warrior (Utilities|Casting|CastToBP_Warrior (Game|Player|GetPlayerPawn 0)))
  (CallFunction|SetAttackTarget _asbp_warrior))

(event EventTick
  (params (DeltaSeconds :type Float%20%28single-precision%29))
  (CallFunction|SetFocusDirection))

(event EventPossess
  (params (PossessedPawn :type Pawn%20Object%20Reference))
  ;[1 1 1] connects isStunned to blackboard
  (bind _asball_chain (Utilities|Casting|CastToBallChain PossessedPawn))
  (bind _output_get (Variables|Default|Setball%20chain _asball_chain))
  (EventDispatchers|BindEventtoStunStateChanged _output_get (delegate Custom|OnStunStateChanged)))

(fn ConstructionScript)

(fn SetAttackTarget
  (params (AttackTarget :type BP%20Warrior%20Object%20Reference))
  (AI|Components|Blackboard|SetValueasObject (Variables|Default|GetBlackboard) (Variables|Default|GetAttackTargetKey) AttackTarget)
  (Variables|Default|SetAttackTarget AttackTarget))

(fn SetFocusDirection
  (bind _ball_chain (Variables|Default|Getball%20chain))
  (Utilities|IsValid (Variables|Default|GetAttackTarget)
    (:Is%20Valid
      (if (and (not (Variables|/Game/Blueprints/BallChain/BallChain.BallChain_C|GetisAttacking (Variables|Default|Getball%20chain))) (not (Variables|/Game/Blueprints/BallChain/BallChain.BallChain_C|GetisStunned (Variables|Default|Getball%20chain))))
        (AI|SetFocalPoint (+ (Transformation|GetActorLocation (Variables|Default|Getball%20chain)) (Math|Vector|MakeVector (.x (Math|Vector|GetForwardVector (Math|Rotator|FindLookatRotation (Transformation|GetActorLocation (Variables|Default|Getball%20chain)) (Transformation|GetActorLocation (Variables|Default|GetAttackTarget))))) 0.0 0.0)))
        (else
          (AI|SetFocalPoint (+ (Transformation|GetActorLocation _ball_chain) (Transformation|GetActorForwardVector _ball_chain)) :!label _label))))
    (:Is%20Not%20Valid
      (goto _label))))