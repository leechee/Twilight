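; AIC_BC is an AI controller that starts the BB_BC blackboard and BT_BC behavior tree on BeginPlay.
; A temporary aggro system then casts the first player pawn to BP_Warrior and passes it to SetAttackTarget.
; SetAttackTarget writes the target to the blackboard's attack target key and stores it in a variable.
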(event EventBeginPlay
  (Class|AIController|UseBlackboard "/Game/Blueprints/AI/BB_BC.BB_BC")
  (AI|RunBehaviorTree "/Game/Blueprints/AI/BT_BC.BT_BC")
  ;[1 1 1] Temporary Aggro System
  (bind _asbp_warrior (Utilities|Casting|CastToBP_Warrior (Game|Player|GetPlayerPawn 0)))
  (CallFunction|SetAttackTarget _asbp_warrior))

(event EventTick
  (params (DeltaSeconds :type Float%20%28single-precision%29)))

(fn ConstructionScript)

(fn SetAttackTarget
  (params (AttackTarget :type BP%20Warrior%20Object%20Reference))
  (AI|Components|Blackboard|SetValueasObject (Variables|Default|GetBlackboard) (Variables|Default|GetAttackTargetKey) AttackTarget)
  (Variables|Default|SetAttackTarget AttackTarget))